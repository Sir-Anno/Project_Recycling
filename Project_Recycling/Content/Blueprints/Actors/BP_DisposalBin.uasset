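; BP_DisposalBin is a sorting bin that scores items deposited into it by matching material type to bin type.
; On overlap it makes the player drop the item, deactivates it if still scorable, and updates GameMode level stats for correct, incorrect or junk deposits.
; A widget shows correct or incorrect feedback, with junk always displayed as incorrect.
; The construction script labels and tints the bin by type through a dynamic material.
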(event OnComponentBeginOverlap(Collisionbox)
  (params (OverlappedComponent :type Primitive%20Component%20Object%20Reference) (OtherActor :type Actor%20Object%20Reference) (OtherComp :type Primitive%20Component%20Object%20Reference) (OtherBodyIndex :type Integer) (bFromSweep :type Boolean) (SweepResult :type Hit%20Result%20Structure%20%28by%20ref%29))
  (bind _gamemoderef (Variables|Default|GetGameModeRef))
  (bind _widget (Variables|Default|GetWidget))
  (bind _leveldetails (Variables|/Game/GameModes/GM_RecycleRamble.GM_RecycleRamble_C|GetLevelDetails _gamemoderef))
  (bind (_level _numberofitemstospawn _itemscorrectlydeposited _itemsincorrectlydeposited) (Utilities|Struct|BreakS_LevelDetails _leveldetails))
  ;[1 1 1] Deposit item
  (bind _asbp_item (Utilities|Casting|CastToBP_Item OtherActor))
  (Variables|Default|SetDepositedItem _asbp_item)
  ;[1 1 1] Force player pawn to drop item
  (bind _asbp_player_pawn (Utilities|Casting|CastToBP_PlayerPawn (Game|Player|GetPlayerPawn 0)))
  (Default|DropItem _asbp_player_pawn)
  ;[1 1 1] Check if item can score - If an item has already been counted and then triggered again this value will be false
  (if (Variables|/Game/Blueprints/Actors/BP_Item.BP_Item_C|GetCan%20score (Variables|Default|GetDepositedItem))
    (Default|SetInactive (Variables|Default|GetDepositedItem))
    ;[1 1 1] Remove item from play
    (if (Utilities|Enum|NotEqual(Enum) (Variables|/Game/Blueprints/Actors/BP_Item.BP_Item_C|GetMaterial%20type (Variables|Default|GetDepositedItem)) "NewEnumerator7")
      (Default|ItemOutOfPlay (Variables|Default|GetGameModeRef))
      ;[1 1 1] Check if deposited item is valid
      (if (Utilities|Enum|Equal(Enum) (Variables|Default|GetBin%20Type) (Variables|/Game/Blueprints/Actors/BP_Item.BP_Item_C|GetMaterial%20type (Variables|Default|GetDepositedItem)))
        ;[1 1 1] Update deposited item stats
        (Math|Integer|IncrementInt _itemscorrectlydeposited ; Correct item
          (:%20%20
            ;[1 1 1] Display icon
            (bind _returnvalue (UserInterface|CreateWidget "/Game/UI/UI_DisposalBin_Display.UI_DisposalBin_Display_C" 0 true))
            (UserInterface|SetWidget _widget _returnvalue)
            (Development|PrintString "Correct Item" true true "(R=0.113357,G=1.000000,B=0.000000,A=1.000000)" 1.0)))
        (else
          (Math|Integer|IncrementInt _itemsincorrectlydeposited ; Incorrect item
            (:%20%20
              (bind _returnvalue_2 (UserInterface|CreateWidget "/Game/UI/UI_DisposalBin_Display.UI_DisposalBin_Display_C" :!label _label))
              (UserInterface|SetWidget _widget _returnvalue_2)
              (Development|PrintString "Incorrect Item" true true "(R=1.000000,G=0.006395,B=0.000000,A=1.000000)" 1.0)))))
      (else
        (Math|Integer|IncrementInt (.Junkdeposited (Utilities|Struct|BreakS_LevelDetails (Variables|/Game/GameModes/GM_RecycleRamble.GM_RecycleRamble_C|GetLevelDetails (Variables|Default|GetGameModeRef))))
          (:%20%20
            (goto _label)))))))

(event EventBeginPlay
  ;[1 1 1] Setup
  (bind _asgm_recycle_ramble (Utilities|Casting|CastToGM_RecycleRamble (Game|GetGameMode)))
  (Variables|Default|SetGameModeRef _asgm_recycle_ramble))

(fn ConstructionScript
  (Rendering|Components|TextRender|SetText (Variables|Default|GetTextRender) (Utilities|Text|ToText(String) (Utilities|String|EnumtoString (Variables|Default|GetBin%20Type))))
  (Utilities|FlowControl|Sequence
    (:then_0
      (switch Utilities|FlowControl|Switch|SwitchonE_ItemTypes (Variables|Default|GetBin%20Type)
        (:NewEnumerator0
          (LocalVariables|SetColour "(R=0.416667,G=0.408149,B=0.314670,A=1.000000)"))
        (:NewEnumerator1
          (LocalVariables|SetColour "(R=0.282986,G=0.282986,B=0.282986,A=1.000000)"))
        (:NewEnumerator2
          (LocalVariables|SetColour "(R=0.000000,G=0.744792,B=0.702924,A=1.000000)"))
        (:NewEnumerator3
          (LocalVariables|SetColour "(R=0.135417,G=0.087563,B=0.059245,A=1.000000)"))
        (:NewEnumerator4
          (LocalVariables|SetColour "(R=0.087970,G=0.776042,B=0.000000,A=1.000000)"))
        (:NewEnumerator5
          (LocalVariables|SetColour "(R=0.654514,G=0.636978,B=0.000000,A=1.000000)"))
        (:NewEnumerator6
          (LocalVariables|SetColour "(R=1.000000,G=0.177900,B=0.000000,A=1.000000)"))
        (:NewEnumerator7
          (LocalVariables|SetColour "(R=0.012153,G=0.012153,B=0.012153,A=1.000000)"))))
    (:then_1
      (bind _returnvalue (Rendering|Material|CreateDynamicMaterialInstance (Variables|Default|GetStaticMesh) 0 "/Game/Assets/Materials/M_Colour.M_Colour" "None" :!class /Script/Engine.PrimitiveComponent))
      (Rendering|Material|SetVectorParameterValue _returnvalue "Colour" (LocalVariables|GetColour) :!class /Script/Engine.MaterialInstanceDynamic))))