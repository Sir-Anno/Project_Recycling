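; BP_ItemKill is a kill volume that removes BP_Item actors from play in Recycle Ramble.
; On box overlap it destroys the item, first reporting it to GM_RecycleRamble as out of play and incrementing the missed count in LevelDetails.
; One excluded MaterialType skips that reporting but is still destroyed.
; The construction script sizes the box from InBoxExtent and rests its base at world Z zero.
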(event OnComponentBeginOverlap(Box)
  (params (OverlappedComponent :type Primitive%20Component%20Object%20Reference) (OtherActor :type Actor%20Object%20Reference) (OtherComp :type Primitive%20Component%20Object%20Reference) (OtherBodyIndex :type Integer) (bFromSweep :type Boolean) (SweepResult :type Hit%20Result%20Structure%20%28by%20ref%29))
  (bind _game_mode_ref (Variables|Default|GetGame%20Mode%20Ref))
  (bind _asbp_item (Utilities|Casting|CastToBP_Item OtherActor))
  (Utilities|FlowControl|Sequence
    (:then_0
      ;[1 1 1] Remove item from play
      (if (Utilities|Enum|NotEqual(Enum) (Variables|/Game/Blueprints/Actors/BP_Item.BP_Item_C|GetMaterial%20type _asbp_item) "NewEnumerator7")
        (Default|ItemOutOfPlay (Variables|Default|GetGame%20Mode%20Ref))
        ;[1 1 1] Update number of missed items
        (bind _result (Math|Integer|IncrementInt (.Itemsmissed (Utilities|Struct|BreakS_LevelDetails (Variables|/Game/GameModes/GM_RecycleRamble.GM_RecycleRamble_C|GetLevelDetails _game_mode_ref))))
          (:%20%20
            (Variables|/Game/GameModes/GM_RecycleRamble.GM_RecycleRamble_C|SetLevelDetails _game_mode_ref (Utilities|Struct|MakeS_LevelDetails (.Level (Utilities|Struct|BreakS_LevelDetails (Variables|/Game/GameModes/GM_RecycleRamble.GM_RecycleRamble_C|GetLevelDetails _game_mode_ref))) (.Numberofitemstospawn (Utilities|Struct|BreakS_LevelDetails (Variables|/Game/GameModes/GM_RecycleRamble.GM_RecycleRamble_C|GetLevelDetails _game_mode_ref))) (.Itemscorrectlydeposited (Utilities|Struct|BreakS_LevelDetails (Variables|/Game/GameModes/GM_RecycleRamble.GM_RecycleRamble_C|GetLevelDetails _game_mode_ref))) (.Itemsincorrectlydeposited (Utilities|Struct|BreakS_LevelDetails (Variables|/Game/GameModes/GM_RecycleRamble.GM_RecycleRamble_C|GetLevelDetails _game_mode_ref))) _result 0 (.Conveyorspeed (Utilities|Struct|BreakS_LevelDetails (Variables|/Game/GameModes/GM_RecycleRamble.GM_RecycleRamble_C|GetLevelDetails _game_mode_ref))) (.Spawnrate (Utilities|Struct|BreakS_LevelDetails (Variables|/Game/GameModes/GM_RecycleRamble.GM_RecycleRamble_C|GetLevelDetails _game_mode_ref)))))
            (Development|PrintString "Item missed" true true "(R=1.000000,G=0.177900,B=0.000000,A=1.000000)")))))
    (:then_1
      (Actor|DestroyActor _asbp_item))))

(event EventBeginPlay
  ;[1 1 1] Setup
  (bind _asgm_recycle_ramble (Utilities|Casting|CastToGM_RecycleRamble (Game|GetGameMode)))
  (Variables|Default|SetGame%20Mode%20Ref _asgm_recycle_ramble))

(fn ConstructionScript
  (bind _returnvalue (Transformation|GetActorLocation))
  (bind _in_box_extent (Variables|Default|GetIn%20Box%20Extent))
  (Components|Box|SetBoxExtent (Variables|Default|GetBox) _in_box_extent true)
  (Transformation|SetWorldLocation (Variables|Default|GetBox) (Math|Vector|MakeVector (.x _returnvalue) (.y _returnvalue) (.Z (Class|KismetMathLibrary|BreakVector3f _in_box_extent))) false false))