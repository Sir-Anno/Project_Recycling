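; Floor catch trigger for the Recycle Ramble game mode that detects items dropped out of play.
; On overlap, an item that can still score is set inactive to prevent double counting.
; One material type counts as deposited junk; others are taken out of play, added to a floor list and counted as missed in the level details.
; The construction script sizes the box and rests its base at world Z zero.
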(event OnComponentBeginOverlap(Box)
  (params (OverlappedComponent :type Primitive%20Component%20Object%20Reference) (OtherActor :type Actor%20Object%20Reference) (OtherComp :type Primitive%20Component%20Object%20Reference) (OtherBodyIndex :type Integer) (bFromSweep :type Boolean) (SweepResult :type Hit%20Result%20Structure%20%28by%20ref%29))
  (bind _asbp_item (Utilities|Casting|CastToBP_Item OtherActor))
  (bind _output_get (Variables|Default|SetItem%20dropped _asbp_item))
  ;[1 1 1] Check if item can score - If an item has already been counted and then triggered again this value will be false
  (if (Variables|/Game/Blueprints/Actors/BP_Item.BP_Item_C|GetCan%20score _output_get)
    (Default|SetInactive _output_get)
    ;[1 1 1] Remove item from play
    (if (Utilities|Enum|NotEqual(Enum) (Variables|/Game/Blueprints/Actors/BP_Item.BP_Item_C|GetMaterial%20type (Variables|Default|GetItem%20dropped)) "NewEnumerator7")
      (Default|ItemOutOfPlay (Variables|Default|GetGame%20Mode%20Ref))
      ;[1 1 1] Add item to list of items on the floor
      (Utilities|Array|AddUnique (Variables|Default|GetItems%20on%20the%20floor) (Variables|Default|GetItem%20dropped))
      ;[1 1 1] Update number of missed items
      (Math|Integer|IncrementInt (.Itemsmissed (Utilities|Struct|BreakS_LevelDetails (Variables|/Game/GameModes/GM_RecycleRamble.GM_RecycleRamble_C|GetLevelDetails (Variables|Default|GetGame%20Mode%20Ref))))
        (:%20%20
          (Development|PrintString "Item missed" true true "(R=1.000000,G=0.177900,B=0.000000,A=1.000000)" 1.0)))
      (else
        (Math|Integer|IncrementInt (.Junkdeposited (Utilities|Struct|BreakS_LevelDetails (Variables|/Game/GameModes/GM_RecycleRamble.GM_RecycleRamble_C|GetLevelDetails (Variables|Default|GetGame%20Mode%20Ref)))))))))

(event EventBeginPlay
  ;[1 1 1] Setup
  (bind _asgm_recycle_ramble (Utilities|Casting|CastToGM_RecycleRamble (Game|GetGameMode)))
  (Variables|Default|SetGame%20Mode%20Ref _asgm_recycle_ramble))

(fn ConstructionScript
  (bind _returnvalue (Transformation|GetActorLocation))
  (bind _in_box_extent (Variables|Default|GetIn%20Box%20Extent))
  (Components|Box|SetBoxExtent (Variables|Default|GetBox) _in_box_extent true)
  (Transformation|SetWorldLocation (Variables|Default|GetBox) (Math|Vector|MakeVector (.x _returnvalue) (.y _returnvalue) (.Z (Class|KismetMathLibrary|BreakVector3f _in_box_extent))) false false))