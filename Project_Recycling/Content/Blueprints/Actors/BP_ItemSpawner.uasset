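; Item spawner for the Recycle Ramble game mode that drops recyclable items and junk into the level.
; It listens for game state changes, enabling spawning at Start Game and starting a timer at the level's spawn rate when In Game.
; While items remain in the game mode's LevelDetails, each tick spawns a random-material BP_Item, decrements the count and adds several junk items, all with randomised X offset and rotation.
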(event Custom|Loop
  (if (> (Utilities|Struct|BreakS_LevelDetails (Variables|/Game/GameModes/GM_RecycleRamble.GM_RecycleRamble_C|GetLevelDetails (Variables|Default|GetGame%20Mode%20Ref))) 0)
    (CallFunction|PickItemType)
    (CallFunction|SpawnItem)
    (CallFunction|DecrementNumberOfItemstoSpawn)
    (CallFunction|SpawnJunk)))

(event Custom|Game%20state%20change
  (params (New%20State :type E_GameStates%20Enum :default "NewEnumerator0"))
  ;[1 1 1] Setup
  (switch Utilities|FlowControl|Switch|SwitchonE_GameStates New%20State
    (:NewEnumerator1
      (Variables|Default|SetCan%20spawn%20items true))
    (:NewEnumerator2
      (CallFunction|SpawnItems))))

(event Custom|Spawn%20items
  (Utilities|Time|SetTimerbyEvent (delegate Custom|Loop) (Utilities|Struct|BreakS_LevelDetails (Variables|/Game/GameModes/GM_RecycleRamble.GM_RecycleRamble_C|GetLevelDetails (Variables|Default|GetGame%20Mode%20Ref))) (Variables|Default|GetCan%20spawn%20items)))

(event EventBeginPlay
  ;[1 1 1] Setup
  (bind _asgm_recycle_ramble (Utilities|Casting|CastToGM_RecycleRamble (Game|GetGameMode)))
  (bind _output_get (Variables|Default|SetGame%20Mode%20Ref _asgm_recycle_ramble))
  (EventDispatchers|AssignEDGameStateChange _output_get (delegate Custom|Game%20state%20change)))

(fn ConstructionScript)

(fn PickItemType
  (switch int (Math|Random|RandomIntegerinRange 0 7)
    (:0
      (Variables|Default|SetItemTypeToSpawn "NewEnumerator0"))
    (:1
      (Variables|Default|SetItemTypeToSpawn "NewEnumerator1"))
    (:2
      (Variables|Default|SetItemTypeToSpawn "NewEnumerator2"))
    (:3
      (Variables|Default|SetItemTypeToSpawn "NewEnumerator3"))
    (:4
      (Variables|Default|SetItemTypeToSpawn "NewEnumerator4"))
    (:5
      (Variables|Default|SetItemTypeToSpawn "NewEnumerator5"))
    (:6
      (Variables|Default|SetItemTypeToSpawn "NewEnumerator6"))))

(fn SpawnItem
  (bind _returnvalue (Transformation|GetActorLocation))
  (bind (_x _y _z) (Class|KismetMathLibrary|BreakVector3f _returnvalue))
  (Game|SpawnActorfromClass "/Game/Blueprints/Actors/BP_Item.BP_Item_C" (Math|Transform|MakeTransform (Math|Vector|MakeVector (Math|Random|RandomFloatinRange -1e+02 1e+02) _y _z) (Math|Rotator|MakeRotator (Math|Random|RandomFloatinRange -45.0 45.0) (Math|Random|RandomFloatinRange -45.0 45.0) (Math|Random|RandomFloatinRange 0.0 1.8e+02)) "1.000000,1.000000,1.000000") "AlwaysSpawn" 0 (Variables|Default|GetItemTypeToSpawn) 0))

(fn DecrementNumberOfItemstoSpawn
  (bind _game_mode_ref (Variables|Default|GetGame%20Mode%20Ref))
  (bind _result (Math|Integer|DecrementInt (.Numberofitemstospawn (Utilities|Struct|BreakS_LevelDetails (Variables|/Game/GameModes/GM_RecycleRamble.GM_RecycleRamble_C|GetLevelDetails _game_mode_ref))))
    (:%20%20
      (Variables|/Game/GameModes/GM_RecycleRamble.GM_RecycleRamble_C|SetLevelDetails _game_mode_ref (Utilities|Struct|MakeS_LevelDetails (.Level (Utilities|Struct|BreakS_LevelDetails (Variables|/Game/GameModes/GM_RecycleRamble.GM_RecycleRamble_C|GetLevelDetails _game_mode_ref))) _result (.Itemscorrectlydeposited (Utilities|Struct|BreakS_LevelDetails (Variables|/Game/GameModes/GM_RecycleRamble.GM_RecycleRamble_C|GetLevelDetails _game_mode_ref))) (.Itemsincorrectlydeposited (Utilities|Struct|BreakS_LevelDetails (Variables|/Game/GameModes/GM_RecycleRamble.GM_RecycleRamble_C|GetLevelDetails _game_mode_ref))) (.Itemsmissed (Utilities|Struct|BreakS_LevelDetails (Variables|/Game/GameModes/GM_RecycleRamble.GM_RecycleRamble_C|GetLevelDetails _game_mode_ref))) 0 (.Conveyorspeed (Utilities|Struct|BreakS_LevelDetails (Variables|/Game/GameModes/GM_RecycleRamble.GM_RecycleRamble_C|GetLevelDetails _game_mode_ref))) 0.0)))))

(fn SpawnJunk
  (bind _returnvalue (Transformation|GetActorLocation))
  (bind (_x _y _z) (Class|KismetMathLibrary|BreakVector3f _returnvalue))
  (for _index (range 1 (Math|Random|RandomIntegerinRange 2 5))
    (Game|SpawnActorfromClass "/Game/Blueprints/Actors/BP_Item.BP_Item_C" (Math|Transform|MakeTransform (Math|Vector|MakeVector (Math|Random|RandomFloatinRange -1e+02 1e+02) _y _z) (Math|Rotator|MakeRotator (Math|Random|RandomFloatinRange -45.0 45.0) (Math|Random|RandomFloatinRange -45.0 45.0) (Math|Random|RandomFloatinRange 0.0 1.8e+02)) "1.000000,1.000000,1.000000") "AlwaysSpawn" 0 "NewEnumerator7" 0)))