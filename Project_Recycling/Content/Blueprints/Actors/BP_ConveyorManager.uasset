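; BP_ConveyorManager moves every BP_Conveyor belt section in the level along its belt direction.
; BeginPlay caches the GM_RecycleRamble game mode, whose LevelDetails supply the conveyor speed.
; Each Tick gathers all conveyors with GetAllActorsOfClass and offsets each along its ArrowComponent's forward vector, scaled by speed and delta time, without sweeping.
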(event EventBeginPlay
  ;[1 1 1] Setup
  (bind _asgm_recycle_ramble (Utilities|Casting|CastToGM_RecycleRamble (Game|GetGameMode)))
  (Variables|Default|SetGM_Ref _asgm_recycle_ramble))

(event EventTick
  (params (DeltaSeconds :type Float%20%28single-precision%29))
  ;[1 1 1] Move all conveyor belt sections
  (bind _outactors (Actor|GetAllActorsOfClass "/Game/Blueprints/Actors/BP_Conveyor.BP_Conveyor_C"))
  (for _array_element _outactors
    (Transformation|AddActorWorldOffset _array_element (* (Math|Vector|GetForwardVector (Actor|GetComponentbyClass _array_element "/Script/Engine.ArrowComponent")) (* DeltaSeconds (.Conveyorspeed (Utilities|Struct|BreakS_LevelDetails (Variables|/Game/GameModes/GM_RecycleRamble.GM_RecycleRamble_C|GetLevelDetails (Variables|Default|GetGM_Ref)))))))))

(fn ConstructionScript)