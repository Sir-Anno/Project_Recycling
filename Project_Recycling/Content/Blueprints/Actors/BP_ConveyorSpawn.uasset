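; BP_ConveyorSpawn is an actor that keeps a conveyor belt going by spawning new BP_Conveyor sections.
; When a section stops overlapping its Box component, it stores that section as LastSection and calls SpawnConveyor.
; SpawnConveyor places the new section at the AttachPoint socket location on that section's mesh, using location only.
; Disconnected LastConveyorSpawned nodes remain in the graph and never run.
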(event OnComponentEndOverlap(Box)
  (params (OverlappedComponent :type Primitive%20Component%20Object%20Reference) (OtherActor :type Actor%20Object%20Reference) (OtherComp :type Primitive%20Component%20Object%20Reference) (OtherBodyIndex :type Integer))
  ;[1 1 1] When conveyor belt section moves out of the way spawn a new section
  (bind _asbp_conveyor (Utilities|Casting|CastToBP_Conveyor OtherActor))
  (Variables|Default|SetLastSection _asbp_conveyor)
  (CallFunction|SpawnConveyor))

(event Custom|Spawn%20Conveyor
  ;[1 1 1] Spawn conveyor belt section
  (Game|SpawnActorfromClass "/Game/Blueprints/Actors/BP_Conveyor.BP_Conveyor_C" (Math|Conversions|ToTransform(Vector) (Transformation|GetSocketLocation (Variables|/Game/Blueprints/Actors/BP_Conveyor.BP_Conveyor_C|GetMesh (Variables|Default|GetLastSection)) "AttachPoint")) "Undefined" 0 0))

(fn ConstructionScript)