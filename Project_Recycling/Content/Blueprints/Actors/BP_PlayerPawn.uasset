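; Player pawn that slides the camera sideways within fixed bounds and lets the mouse drag physics items around.
; Click traces from the cursor and grabs a pickable BP_Item with a PhysicsHandle, notifying the item when held and released.
; Tick moves the handle target along the cursor ray at the original hit distance.
; The construction script sets spring arm length and pitch from camera variables.
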(event Custom|Drop%20item
  ;[1 1 1] Drop item
  (Physics|Components|PhysicsHandle|ReleaseComponent (Variables|Default|GetPhysicsHandle))
  (bind _asbp_item (Utilities|Casting|CastToBP_Item (Components|GetOwner (Variables|Default|GetGrabbedComponent))))
  (Default|IsHeld? _asbp_item false))

(event EventTick
  (params (DeltaSeconds :type Float%20%28single-precision%29))
  (bind _returnvalue (Game|GetPlayerController 0))
  (bind (_worldlocation _worlddirection) (Game|Player|ConvertMouseLocationToWorldSpace _returnvalue))
  ;[1 1 1] Update held items location
  (Variables|Default|SetDelta%20Seconds DeltaSeconds)
  (Physics|Components|PhysicsHandle|SetTargetLocation (Variables|Default|GetPhysicsHandle) (+ _worldlocation (* _worlddirection (Variables|Default|GetOriginalDistanceToObject)))))

(event Input|ActionEvents|InputActionClick
  (params (Key :type Key%20Structure :default "None"))
  (bind _returnvalue (Game|GetPlayerController 0))
  (bind (_worldlocation _worlddirection) (Game|Player|ConvertMouseLocationToWorldSpace _returnvalue))
  ;[1 1 1] Pick up / drop item
  (:Pressed
    (bind _outhit (Collision|LineTraceByChannel _worldlocation (+ _worldlocation (* _worlddirection (Variables|Default|GetReachDistance))) "TraceTypeQuery1" false 0 "None" true "(R=1.000000,G=0.000000,B=0.000000,A=1.000000)" "(R=0.000000,G=1.000000,B=0.000000,A=1.000000)" 1.0)) ; Fire a laser
    (bind _asbp_item (Utilities|Casting|CastToBP_Item (.HitActor (Collision|BreakHitResult _outhit)))) ; Did we hit an item?
    (if (Variables|/Game/Blueprints/Actors/BP_Item.BP_Item_C|GetCan%20be%20picked%20up _asbp_item)
      (bind _output_get (Variables|Default|SetGrabbedComponent (.HitComponent (Collision|BreakHitResult _outhit)))) ; Set items mesh as grabbed component
      (Variables|Default|SetOriginalDistanceToObject (.Distance (Collision|BreakHitResult _outhit)))
      (if (Physics|IsSimulatingPhysics _output_get "None")
        (Class|PhysicsHandleComponent|GrabComponentatLocation (Variables|Default|GetPhysicsHandle) (Variables|Default|GetGrabbedComponent) "None" (.Location (Collision|BreakHitResult _outhit))) ; Grab the item at the location the mouse hit on the mesh
        ;[1 1 1] Tell item its being picked up
        (bind _asbp_item_2 (Utilities|Casting|CastToBP_Item (Components|GetOwner (Variables|Default|GetGrabbedComponent))))
        (Default|IsHeld? _asbp_item_2 true))))
  (:Released
    (bind _asbp_item_3 (Utilities|Casting|CastToBP_Item (.HitActor (Collision|BreakHitResult _outhit))))
    (if (Variables|/Game/Blueprints/Actors/BP_Item.BP_Item_C|GetCan%20be%20picked%20up _asbp_item_3)
      (CallFunction|DropItem))))

(event Input|AxisEvents|InputAxisMove
  (params (AxisValue :type Float%20%28single-precision%29))
  (bind _returnvalue (Transformation|GetActorLocation))
  ;[1 1 1] Move camera left / right
  (Transformation|SetActorLocation (Math|Vector|MakeVector (.x _returnvalue) (Math|Float|Clamp(Float) (+ (* (* AxisValue (Variables|Default|GetMovementSpeed)) (Variables|Default|GetDelta%20Seconds)) (.y _returnvalue)) -7e+02 7e+02) (.z _returnvalue)) false false))

(fn ConstructionScript
  (Variables|/Script/Engine.SpringArmComponent|SetTargetArmLength (Variables|Default|GetSpringArm) (Variables|Default|GetCameraDistance))
  (Transformation|SetRelativeRotation (Variables|Default|GetSpringArm) (Math|Rotator|MakeRotator 0.0 (Variables|Default|GetCameraRotation) 0.0) false false))