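; BP_Item is a holdable waste item typed by material, with a scoring flag that can be switched off.
; The construction script picks a random mesh from that material's pool, setting its scale and highlight stencil.
; Pickup and impact sounds follow material, with drop sounds throttled and limited by a bounce counter reset on release.
; Cursor hover outlines unheld items via custom depth, and hitting the "Floor" actor shows a one-time error widget.
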(event OnComponentHit(Mesh)
  (params (HitComponent :type Primitive%20Component%20Object%20Reference) (OtherActor :type Actor%20Object%20Reference) (OtherComp :type Primitive%20Component%20Object%20Reference) (NormalImpulse :type Vector :default "0, 0, 0") (Hit :type Hit%20Result%20Structure%20%28by%20ref%29))
  (bind (_bblockinghit _binitialoverlap _time _distance _location _impactpoint _normal _impactnormal _physmat _hitactor) (Collision|BreakHitResult Hit))
  ;[1 1 1] Display warning widget when item is dropped on floor
  (bind _asstatic_mesh_actor (Utilities|Casting|CastToStaticMeshActor _hitactor))
  (if (== (Utilities|String|StringToName (Utilities|GetDisplayName _asstatic_mesh_actor)) "Floor")
    (Utilities|FlowControl|DoOnce false
      (:Completed
        (Transformation|SetWorldLocation (Variables|Default|GetWidget) _impactpoint false false)
        (bind _returnvalue (UserInterface|CreateWidget "/Game/UI/UI_Error.UI_Error_C"))
        (UserInterface|SetWidget (Variables|Default|GetWidget) _returnvalue)))))

(event OnBeginCursorOver(Mesh)
  (params (TouchedComponent :type Primitive%20Component%20Object%20Reference))
  (bind _mesh (Variables|Default|GetMesh))
  ;[1 1 1] Enable/disable post process effect when mouse overed
  (if (not (Variables|Default|GetIs%20Held))
    (Rendering|SetRenderCustomDepth _mesh true)
    (Rendering|SetCustomDepthStencilValue _mesh (Variables|Default|GetHighlight%20value))))

(event OnEndCursorOver(Mesh)
  (params (TouchedComponent :type Primitive%20Component%20Object%20Reference))
  ;[1 1 1] Enable/disable post process effect when mouse overed
  (Rendering|SetRenderCustomDepth (Variables|Default|GetMesh) false))

(event Custom|Is%20held?
  (params (Is%20held? :type Boolean))
  ;[1 1 1] Play pick up sound effects
  (bind _output_get (Variables|Default|SetIs%20Held Is%20held?))
  (if _output_get
    (switch Utilities|FlowControl|Switch|SwitchonE_ItemTypes (Variables|Default|GetMaterial%20type)
      (:NewEnumerator0
        (Variables|Default|SetSound%20to%20play "/Game/Assets/Sounds/Cues/SC_PaperPickup.SC_PaperPickup"))
      (:NewEnumerator1
        (Variables|Default|SetSound%20to%20play "/Game/Assets/Sounds/Cues/SC_MetalPickup.SC_MetalPickup"))
      (:NewEnumerator2
        (Variables|Default|SetSound%20to%20play "/Game/Assets/Sounds/Cues/SC_GlassPickup.SC_GlassPickup"))
      (:NewEnumerator3
        (Variables|Default|SetSound%20to%20play "/Game/Assets/Sounds/Cues/SC_PlasticPickup.SC_PlasticPickup"))
      (:NewEnumerator4
        (Variables|Default|SetSound%20to%20play "/Game/Assets/Sounds/Cues/SC_OrganicPickup.SC_OrganicPickup"))
      (:NewEnumerator5
        (Variables|Default|SetSound%20to%20play "/Game/Assets/Sounds/Cues/SC_BatteryPickup.SC_BatteryPickup"))
      (:NewEnumerator6
        (Variables|Default|SetSound%20to%20play 0))
      (:NewEnumerator7
        (Variables|Default|SetSound%20to%20play "/Game/Assets/Sounds/Cues/SC_JunkPickup.SC_JunkPickup")))
    (Audio|PlaySound2D (Variables|Default|GetSound%20to%20play) 1.0 1.0 0.0 0 0 false)
    (else
      (Variables|Default|SetBounce%20count 3)
      (CallFunction|ResetNoise))))

(event Custom|Set%20inactive
  (Variables|Default|SetCan%20score false))

(event Custom|Reset%20noise
  ;[1 1 1] Play drop sound effects
  (Utilities|FlowControl|DoOnce false) ; enters at Reset
)

(event Collision|EventHit
  (params (MyComp :type Primitive%20Component%20Object%20Reference) (Other :type Actor%20Object%20Reference) (OtherComp :type Primitive%20Component%20Object%20Reference) (bSelfMoved :type Boolean) (HitLocation :type Vector :default "0, 0, 0") (HitNormal :type Vector :default "0, 0, 0") (NormalImpulse :type Vector :default "0, 0, 0") (Hit :type Hit%20Result%20Structure%20%28by%20ref%29))
  ;[1 1 1] Play drop sound effects
  (Variables|Default|SetActor%20hit Other)
  (Utilities|FlowControl|DoOnce false
    (:Completed
      (if (> (Variables|Default|GetBounce%20count) 0)
        (switch Utilities|FlowControl|Switch|SwitchonE_ItemTypes (Variables|Default|GetMaterial%20type)
          (:NewEnumerator0
            (Variables|Default|SetSound%20to%20play "/Game/Assets/Sounds/Cues/SC_PaperDrop.SC_PaperDrop"))
          (:NewEnumerator1
            (Variables|Default|SetSound%20to%20play "/Game/Assets/Sounds/Cues/SC_MetalDrop.SC_MetalDrop"))
          (:NewEnumerator2
            (Variables|Default|SetSound%20to%20play "/Game/Assets/Sounds/Cues/SC_GlassDrop.SC_GlassDrop"))
          (:NewEnumerator3
            (Variables|Default|SetSound%20to%20play "/Game/Assets/Sounds/Cues/SC_PlasticDrop.SC_PlasticDrop"))
          (:NewEnumerator4
            (Variables|Default|SetSound%20to%20play "/Game/Assets/Sounds/Cues/SC_OrganicDrop.SC_OrganicDrop"))
          (:NewEnumerator5
            (Variables|Default|SetSound%20to%20play 0))
          (:NewEnumerator6
            (Variables|Default|SetSound%20to%20play 0))
          (:NewEnumerator7
            (Variables|Default|SetSound%20to%20play "/Game/Assets/Sounds/Cues/SC_JunkDrop.SC_JunkDrop")))
        (Audio|PlaySoundatLocation (Variables|Default|GetSound%20to%20play) HitLocation "0, 0, 0" 1.0 1.0 0.0 0 0 0 0)
        ;[1 1 1] Reset noise
        (Utilities|FlowControl|Delay 0.2)
        (CallFunction|ResetNoise)
        (Math|Integer|DecrementInt (Variables|Default|GetBounce%20count))))))

(fn ConstructionScript
  (Utilities|FlowControl|Sequence
    (:then_0
      (switch Utilities|FlowControl|Switch|SwitchonE_ItemTypes (Variables|Default|GetMaterial%20type)
        (:NewEnumerator0
          (Variables|Default|SetHighlight%20value 1)
          (bind _output_get (LocalVariables|SetNewMesh (.OutItem (Utilities|Array|Random (Variables|Default|GetPaper%20mesh%20pool)))))
          (Components|StaticMesh|SetStaticMesh (Variables|Default|GetMesh) _output_get)
          (if (== _output_get "/Game/Assets/Meshes/PizzaBox.PizzaBox")
            (LocalVariables|SetSpawnScale 0.25)
            (else
              (LocalVariables|SetSpawnScale 2.0))))
        (:NewEnumerator1
          (Variables|Default|SetHighlight%20value 2)
          (bind _output_get_2 (LocalVariables|SetNewMesh (.OutItem (Utilities|Array|Random (Variables|Default|GetMetal%20mesh%20pool)))))
          (Components|StaticMesh|SetStaticMesh (Variables|Default|GetMesh) _output_get_2)
          (LocalVariables|SetSpawnScale 2.0))
        (:NewEnumerator2
          (Variables|Default|SetHighlight%20value 3)
          (bind _output_get_3 (LocalVariables|SetNewMesh (.OutItem (Utilities|Array|Random (Variables|Default|GetGlass%20mesh%20pool)))))
          (Components|StaticMesh|SetStaticMesh (Variables|Default|GetMesh) _output_get_3)
          (LocalVariables|SetSpawnScale 2.0))
        (:NewEnumerator3
          (Variables|Default|SetHighlight%20value 4)
          (bind _output_get_4 (LocalVariables|SetNewMesh (.OutItem (Utilities|Array|Random (Variables|Default|GetPlastic%20mesh%20pool)))))
          (Components|StaticMesh|SetStaticMesh (Variables|Default|GetMesh) _output_get_4)
          (LocalVariables|SetSpawnScale 2.0))
        (:NewEnumerator4
          (Variables|Default|SetHighlight%20value 5)
          (bind _output_get_5 (LocalVariables|SetNewMesh (.OutItem (Utilities|Array|Random (Variables|Default|GetOrganic%20mesh%20pool)))))
          (Components|StaticMesh|SetStaticMesh (Variables|Default|GetMesh) _output_get_5)
          (LocalVariables|SetSpawnScale 0.1))
        (:NewEnumerator5
          (Variables|Default|SetHighlight%20value 6)
          (bind _output_get_6 (LocalVariables|SetNewMesh (.OutItem (Utilities|Array|Random (Variables|Default|GetBatteries%20mesh%20pool)))))
          (Components|StaticMesh|SetStaticMesh (Variables|Default|GetMesh) _output_get_6)
          (if (== _output_get_6 "/Game/Assets/Meshes/CarBattery.CarBattery")
            (LocalVariables|SetSpawnScale 0.75)
            (else
              (LocalVariables|SetSpawnScale 1.0))))
        (:NewEnumerator6
          (Variables|Default|SetHighlight%20value 7)
          (bind _output_get_7 (LocalVariables|SetNewMesh (.OutItem (Utilities|Array|Random (Variables|Default|GetE-Waste%20mesh%20pool)))))
          (Components|StaticMesh|SetStaticMesh (Variables|Default|GetMesh) _output_get_7)
          (LocalVariables|SetSpawnScale 2.0))
        (:NewEnumerator7
          (Variables|Default|SetHighlight%20value 8)
          (bind _output_get_8 (LocalVariables|SetNewMesh (.OutItem (Utilities|Array|Random (Variables|Default|GetJunk%20mesh%20pool)))))
          (Components|StaticMesh|SetStaticMesh (Variables|Default|GetMesh) _output_get_8)
          (if (or (== _output_get_8 "/Game/Assets/Meshes/Trash/TrashBag.TrashBag") (== _output_get_8 "/Game/Assets/Meshes/Trash/TrashBag2.TrashBag2"))
            (LocalVariables|SetSpawnScale 0.5)
            (else
              (LocalVariables|SetSpawnScale 1.0)))))
      (Transformation|SetWorldScale3D (Variables|Default|GetMesh) (* "1.000000,1.000000,1.000000" (LocalVariables|GetSpawnScale))))))