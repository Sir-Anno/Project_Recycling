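; Game mode for Recycle Ramble, a conveyor item-sorting game, running each level through Setup, Start Game, In Game and End Game states.
; Setup loads level details from a data table row named by the URL "Level" option, falling back to "Test".
; A repeating one-second check ends the game when no items remain in play.
; It also handles pausing, computes a letter grade from deposits and misses, and prints debug stats every tick.
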(event Custom|Item%20out%20of%20play
  ;[1 1 1] Update items in play
  (Math|Integer|DecrementInt (Variables|Default|GetItems%20in%20play)))

(event Custom|Toggle%20Pause%20Game
  (params (Pause :type Boolean))
  ;[1 1 1] Pause / Unpause game
  (Game|SetGamePaused Pause)
  (Default|CallEDPauseGame))

(event Custom|Start%20Game
  ;[1 1 1] Game states
  (Input|SetInputModeGameandUI (Game|GetPlayerController 0) 0 "DoNotLock" false)
  (CallFunction|ChangeGameState "NewEnumerator2"))

(event Custom|Setup
  (bind _leveldetails (Variables|Default|GetLevelDetails))
  (bind _numberofitemstospawn (Utilities|Struct|BreakS_LevelDetails _leveldetails))
  ;[1 1 1] Game states
  (CallFunction|SetupLevelDetails)
  (Input|SetInputModeUIOnly (Game|GetPlayerController 0) 0 "DoNotLock")
  (bind _returnvalue (UserInterface|CreateWidget "/Game/UI/UI_HowToPlay.UI_HowToPlay_C"))
  (UserInterface|Viewport|AddtoViewport _returnvalue 0)
  (Variables|Default|SetTotalLevelItems (Math|Conversions|ToFloat(Integer) _numberofitemstospawn))
  (Variables|Default|SetItems%20in%20play _numberofitemstospawn))

(event Custom|In%20Game
  ;[1 1 1] Game states
  (bind _returnvalue (Utilities|Time|SetTimerbyEvent (delegate Custom|In%20Game) 1.0))
  (bind _all_items_used (CallFunction|CheckAllItemsUsed))
  (if _all_items_used
    (Utilities|Time|ClearandInvalidateTimerbyHandle _returnvalue)
    (CallFunction|ChangeGameState "NewEnumerator3")))

(event Custom|End%20Game
  ;[1 1 1] Game states
  (Utilities|FlowControl|Delay 2.0)
  (bind _asbp_player_pawn (Utilities|Casting|CastToBP_PlayerPawn (Game|Player|GetPlayerPawn 0)))
  (Default|DropItem _asbp_player_pawn) ; Force the player pawn to drop \nany held item when the game ends
  (Input|DisableInput _asbp_player_pawn (Game|GetPlayerController 0)) ; Stops player pawn moving \nwhen game ends
  (bind _returnvalue (UserInterface|CreateWidget "/Game/UI/UI_GameOver.UI_GameOver_C"))
  (UserInterface|Viewport|AddtoViewport _returnvalue 0)
  (Input|SetInputModeUIOnly (Game|GetPlayerController 0) 0 "DoNotLock"))

(event Custom|Change%20Game%20State
  (params (New%20state :type E_GameStates%20Enum :default "E_GameStates_MAX"))
  ;[1 1 1] Change game state
  (Default|CallEDGameStateChange New%20state)
  (switch Utilities|FlowControl|Switch|SwitchonE_GameStates New%20state
    (:NewEnumerator0
      (CallFunction|Setup))
    (:NewEnumerator1
      (CallFunction|StartGame))
    (:NewEnumerator2
      (CallFunction|InGame))
    (:NewEnumerator3
      (CallFunction|EndGame))))

(event EventBeginPlay
  ;[1 1 1] Begin play
  (CallFunction|ChangeGameState "NewEnumerator0"))

(event EventTick
  (params (DeltaSeconds :type Float%20%28single-precision%29))
  (bind _leveldetails (Variables|Default|GetLevelDetails))
  (bind (_level _numberofitemstospawn _itemscorrectlydeposited _itemsincorrectlydeposited _itemsmissed _junkdeposited _conveyorspeed _spawnrate) (Utilities|Struct|BreakS_LevelDetails _leveldetails))
  ;[1 0.6748 0] Debugging
  (bind _grade (CallFunction|CalculateGrade))
  (Development|PrintString (Utilities|String|Append "Level: #" (Utilities|String|ToString(Integer) _level) " 
Items left to spawn: " (Utilities|String|ToString(Integer) _numberofitemstospawn) " 
Correctly deposited: " (Utilities|String|ToString(Integer) _itemscorrectlydeposited) " 
Incorrectly deposited: " (Utilities|String|ToString(Integer) _itemsincorrectlydeposited) " 
Missed: " (Utilities|String|ToString(Integer) _itemsmissed) " 
Conveyor speed: " (Utilities|String|ToString(Float) _conveyorspeed) " 
Spawn rate: " (Utilities|String|ToString(Float) _spawnrate) " 
Junk deposited: " (Utilities|String|ToString(Integer) _junkdeposited) " 
Current grade: " _grade) true true "(R=0.000000,G=0.660000,B=1.000000,A=1.000000)" DeltaSeconds))

(fn ConstructionScript)

(fn CheckAllItemsUsed
  (if (== (Variables|Default|GetItems%20in%20play) 0)
    (return true)
    (else
      (return false))))

(fn SetupLevelDetails
  (bind _returnvalue (Utilities|GetDataTableRow (Variables|Default|GetDataTable) (Utilities|String|StringToName (Class|GameplayStatics|ParseOption (Variables|/Script/Engine.GameModeBase|GetOptionsString (Game|GetGameMode)) "Level")))
    (:then
      (Variables|Default|SetLevelDetails _returnvalue)
      (Development|PrintString "DATA TABLE OPTIONS LOADED SUCCESSFULLY" true true "(R=0.087970,G=0.776042,B=0.000000,A=1.000000)"))
    (:RowNotFound
      (Development|PrintString "DATA TABLE NOT LOADED 
DEFAULTING TO TEST LEVEL" true true "(R=1.000000,G=0.000000,B=0.000000,A=1.000000)")
      (bind _returnvalue_2 (Utilities|GetDataTableRow (Variables|Default|GetDataTable) "Test")
        (:then
          (Variables|Default|SetLevelDetails _returnvalue_2))))))

(fn CalculateGrade
  (bind _leveldetails (Variables|Default|GetLevelDetails))
  (bind _gradebands (LocalVariables|GetGradeBands))
  (bind (_level _numberofitemstospawn _itemscorrectlydeposited _itemsincorrectlydeposited _itemsmissed) (Utilities|Struct|BreakS_LevelDetails _leveldetails))
  (bind (_s _a _b _c _d _f) (Utilities|Struct|BreakS_GradingBands _gradebands))
  ;[1 0 0] I don't understand maths :/
  (LocalVariables|SetTotalScoreAvaliable (* (Variables|Default|GetTotalLevelItems) 5))
  (bind _output_get (LocalVariables|SetUserScore (Math|Conversions|ToFloat(Integer) (- (* _itemscorrectlydeposited 5) (+ (* _itemsincorrectlydeposited 5) (* _itemsmissed 3))))))
  (LocalVariables|SetFinalScorePercent (* (/ _output_get (LocalVariables|GetTotalScoreAvaliable)) 1e+02))
  (if (== (LocalVariables|GetFinalScorePercent) _s)
    (return "S")
    (elif (and (>= (LocalVariables|GetFinalScorePercent) _a) (< (LocalVariables|GetFinalScorePercent) (- _s 1)))
      (return "A")
      (elif (and (>= (LocalVariables|GetFinalScorePercent) _b) (< (LocalVariables|GetFinalScorePercent) (- _a 1)))
        (return "B")
        (elif (and (>= (LocalVariables|GetFinalScorePercent) _c) (< (LocalVariables|GetFinalScorePercent) (- _b 1)))
          (return "C")
          (elif (and (>= (LocalVariables|GetFinalScorePercent) _d) (< (LocalVariables|GetFinalScorePercent) (- _c 1)))
            (return "D")
            (elif (< (LocalVariables|GetFinalScorePercent) _f)
              (return "F"))))))))